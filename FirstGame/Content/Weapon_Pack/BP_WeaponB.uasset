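; Melee weapon actor that attaches to a character and damages what it overlaps.
; AttachToCharacter stores the wielder and snaps the weapon to the "Axe" socket on its mesh.
; DoDamage scans the Weapon component's overlapping actors, applies fixed damage to the first that isn't the wielder, then returns.
; The event graph is empty; NotUsing functions keep disconnected experiments, including box-trace, radial and point damage.
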(event Custom|AttachToCharacter_1_1
  (params (Character :type Character%20Object%20Reference) (result :type Boolean)))

(event EventBeginPlay)

(event Collision|EventActorBeginOverlap
  (params (OtherActor :type Actor%20Object%20Reference)))

(event EventTick
  (params (DeltaSeconds :type Float%20%28single-precision%29)))

(fn ConstructionScript)

(fn NotUsingThistoo
  (params (Character :type Character%20Object%20Reference)))

(fn NotUsingThisfunction)

(fn AttachtoCharacter
  (params (Character :type Character%20Object%20Reference))
  (bind _output_get (Variables|Default|Setcharacter Character))
  (bind _returnvalue (Transformation|AttachComponentToComponent (Variables|/Script/Engine.Character|GetMesh _output_get) "Axe" "SnapToTarget" "SnapToTarget" "KeepWorld" true))
  (return _returnvalue))

(fn DoDamage
  (bind _character (Variables|Default|Getcharacter))
  (for _array_element (Collision|GetOverlappingActors (Variables|Default|Getweapon) 0 :!class /Script/Engine.PrimitiveComponent)
    (if (!= _array_element _character)
      ;[0.15 0.15 0.15 0.5] Base Damage- 가할 데미지
      ; Event Instigator- 가해자 플레이어 컨트롤러
      ; Damage Causer-가해자 흉기
      ; Damage TypecClass-불,물, 번개,출혈, 독 등
      (Game|Damage|ApplyDamage _array_element 1.2e+02 (Pawn|GetController _character) self "/Script/Engine.DamageType")
      (return false))))