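; BP_Dummy is a damageable target dummy with a name and HP tag that shatters when its HP runs out.
; On BeginPlay it loads its stats from DT_MonsterData by RowName and creates a viewport name tag widget.
; AnyDamage subtracts raw damage from current HP and refreshes the tag.
; On death it crumbles its Geometry Collection with a radial impulse, removes the tag and destroys itself after a delay.
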(event Collision|EventActorBeginOverlap
  (params (OtherActor :type Actor%20Object%20Reference)))

(event EventTick
  (params (DeltaSeconds :type Float%20%28single-precision%29)))

(event Game|Damage|EventAnyDamage
  (params (Damage :type Float%20%28single-precision%29) (DamageType :type Damage%20Type%20Object%20Reference) (InstigatedBy :type Controller%20Object%20Reference) (DamageCauser :type Actor%20Object%20Reference))
  ;[0.15 0.15 0.15 0.5] 피해자 이벤트
  ; 번개모양아이콘- 네트워크 상황에 동작 가능
  (Development|PrintString (Utilities|String|Append "AnyDamage" "Damage:" (Utilities|String|ToString(Float) Damage) ".instigated by" (Utilities|GetDisplayName InstigatedBy) "damage causer" (Utilities|GetDisplayName DamageCauser)))
  (bind _isjustdead (CallFunction|AddDamage Damage))
  (if _isjustdead
    (CallFunction|DoDeath)))

(event EventBeginPlay
  (Utilities|FlowControl|Sequence
    (:then_0
      ;[0.15 0.15 0.15 0.5] 데이터테이블 가져오기
      ; 1. 가져온 데이터 테이블에서 구조체 선택
      ; 2. 선택한 구조체를 현재 상태에 업데이트
      (bind _returnvalue (Utilities|GetDataTableRow "/Game/Weapon_Pack/DT_MonsterData.DT_MonsterData" (Variables|Default|GetRow%20Name))
        (:then
          (Utilities|Struct|SetmembersinST_CurMonsState (Variables|Default|GetCurMonState) (Utilities|Struct|MakeST_MonsterState (.Name (Utilities|Struct|BreakST_MonsterState _returnvalue)) (.MaxHP (Utilities|Struct|BreakST_MonsterState _returnvalue)) (.Def (Utilities|Struct|BreakST_MonsterState _returnvalue))) (.MaxHP (Utilities|Struct|BreakST_MonsterState _returnvalue))))))
    (:then_1
      ;[0.15 0.15 0.15 0.5] 위젯에 표시
      (CallFunction|CreateNameTag))))

(fn ConstructionScript)

(fn CreateNameTag
  (bind _returnvalue (UserInterface|CreateWidget "/Game/Weapon_Pack/BP_NameTagWidget.BP_NameTagWidget_C" 0 self))
  (bind _output_get (Variables|Default|SetNameTag _returnvalue))
  (UserInterface|Viewport|AddtoViewport _output_get 0)
  (CallFunction|UpdateHP)
  (CallFunction|UpdateName))

(fn AddDamage
  (params (Damage :type Float%20%28double-precision%29))
  (if (CallFunction|IsDeath)
    ;[0.15 0.15 0.15 0.5] Comment
    (return false)
    (else
      ;[0.15 0.15 0.15 0.5] 현재 HP STATE에  저장
      (Utilities|Struct|SetmembersinST_CurMonsState (Variables|Default|GetCurMonState) (- (.curhp (Variables|Default|GetCurMonState)) Damage))
      ;[0.15 0.15 0.15 0.5] 초기값 저장
      (CallFunction|UpdateHP)
      (if (CallFunction|IsDeath)
        (return true)))))

(fn DoDeath
  (bind _geometrycollection (Variables|Default|GetGeometryCollection))
  ;[0.15 0.15 0.15 0.5] Comment
  (Class|GeometryCollectionComponent|CrumbleActiveClusters _geometrycollection)
  ;;[0.15 0.15 0.15 0.5] 방사형으로 힘을 줌
  (Physics|AddRadialImpulse _geometrycollection (+ (Transformation|GetWorldLocation _geometrycollection) "0.000000,0.000000,30.000000") 1e+01 1e+02 "RIF_Constant" false)
  (Utilities|Time|SetTimerbyFunctionName 0 "DoDestroy" 5.0)
  (Widget|RemovefromParent (Variables|Default|GetNameTag)))

(fn DoDestroy
  (Actor|DestroyActor))

(fn UpdateHP
  (bind _curmonstate (Variables|Default|GetCurMonState))
  (Default|SetHPWidget (Variables|Default|GetNameTag) (.curhp _curmonstate) (.maxhp (.state _curmonstate)))
  (return))

(fn IsDeath
  (return (<= (.curhp (Variables|Default|GetCurMonState)) 0.0)))

(fn UpdateName
  (Default|SetNameTagName (Variables|Default|GetNameTag) (.name (.state (Variables|Default|GetCurMonState)))))

(fn GetNameTagHP
  (bind _curmonstate (Variables|Default|GetCurMonState))
  (return (.curhp _curmonstate) (.maxhp (.state _curmonstate))))

(fn GetNameTagLocation
  (return (Transformation|GetWorldLocation (Variables|Default|GetNameTagLoc))))

(fn GetNameTagName
  (return (.name (.state (Variables|Default|GetCurMonState)))))