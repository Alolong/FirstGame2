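; Base weapon actor that a character can equip, drop, attack with and use to deal damage.
; Attaching stores the wielder and snaps the weapon to a mesh socket with physics off; detaching reverses this.
; DoAttack plays the wielder's montage, while DoDamage box-traces between two blade sockets, ignoring the wielder, and returns after damaging the first hit.
; DoDamagef holds only unconnected damage experiments, and Attachtochar is a simpler hardcoded-socket attach variant.
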(event EventBeginPlay)

(event Collision|EventActorBeginOverlap
  (params (OtherActor :type Actor%20Object%20Reference)))

(event EventTick
  (params (DeltaSeconds :type Float%20%28single-precision%29)))

(fn ConstructionScript)

(fn Attachtochar
  (params (Character :type Character%20Object%20Reference))
  (bind _output_get (Variables|Default|Setcharacter Character))
  (Transformation|AttachComponentToComponent (Variables|/Script/Engine.Character|GetMesh _output_get) "Sword" "SnapToTarget" "SnapToTarget" "KeepWorld" true))

(fn DoDamagef)

(fn AttachtoCharacter
  (params (Character :type Character%20Object%20Reference))
  ;[0.15 0.15 0.15 0.5] 캐릭터
  (bind _output_get (Variables|Default|Setcharacter Character))
  ;[0.15 0.15 0.15 0.5] 장착 전에 시뮬끄기
  (Physics|SetSimulatePhysics (Variables|Default|Getweapon) false)
  ;[0.15 0.15 0.15 0.5] 장착
  (bind _returnvalue (Transformation|AttachComponentToComponent (Variables|/Script/Engine.Character|GetMesh _output_get) (Variables|Default|GetSocket%20Name) "SnapToTarget" "SnapToTarget" "KeepWorld" true))
  (return _returnvalue))

(fn DetachtoCharacter
  (params (Character :type Character%20Object%20Reference))
  ;[0.15 0.15 0.15 0.5] Attach와 역순
  ;;[0.15 0.15 0.15 0.5] 탈착
  (Transformation|DetachFromActor "KeepWorld" "KeepWorld" "KeepWorld")
  ;;[0.15 0.15 0.15 0.5] 시뮬
  (Physics|SetSimulatePhysics (Variables|Default|Getweapon) true)
  ;;[0.15 0.15 0.15 0.5] 캐릭터
  (Variables|Default|Setcharacter 0)
  (return false))

(fn DoAttack
  (Animation|PlayAnimMontage (Variables|Default|Getcharacter) "/Game/Characters/Mannequins/Animations/Attack/Animon_AttackTest.Animon_AttackTest" 1.0 "None")
  (return false))

(fn DoDamage
  (bind _weapon (Variables|Default|Getweapon))
  (bind _outhits (Class|KismetSystemLibrary|BoxTraceMultiforObjects (Transformation|GetSocketLocation _weapon "HitA") (Transformation|GetSocketLocation _weapon "HitB") "1.000000,1.000000,1.000000" "0, 0, 0" (Utilities|Array|MakeArray "ObjectTypeQuery1" "ObjectTypeQuery2" "ObjectTypeQuery4" "ObjectTypeQuery5" "ObjectTypeQuery6") false (Utilities|Array|MakeArray (Variables|Default|Getcharacter)) "ForDuration" true))
  (for _array_element _outhits
    (Game|Damage|ApplyDamage (.HitActor (Collision|BreakHitResult _array_element)) 1.2e+02 (Pawn|GetController (Variables|Default|Getcharacter)) self "/Script/Engine.DamageType")
    (return false)))